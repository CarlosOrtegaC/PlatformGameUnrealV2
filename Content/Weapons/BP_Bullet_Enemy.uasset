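; Enemy bullet projectile that damages the player on overlap.
; Tick moves it forward along its facing at a Speed value, without sweep, so hits rely on overlap events.
; Overlapping BP_ThirdPersonCharacter calls that character's damage event directly with a fixed amount, plays a hit sound and destroys the bullet.
; A timer started on BeginPlay destroys it after a few seconds.
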(event `self.ReceiveActorBeginOverlap`
  (params (OtherActor :type "Actor Object Reference"))
  ;[1 1 1] Aparición bala + sonido
  (bind _asbp_third_person_character (cast `/Game/ThirdPerson/Blueprints/BP_ThirdPersonCharacter` OtherActor))
  (`/Game/ThirdPerson/Blueprints/BP_ThirdPersonCharacter.OnTakeAnyDamage_Event_0` _asbp_third_person_character null 5.0 null null null)
  (`GameplayStatics.PlaySoundAtLocation` "/Game/Audio/ShootPlayerDmg.ShootPlayerDmg" (0.0 0.0 0.0) (struct) 0.5 1.0 0.0 null null null null)
  (`self.K2_DestroyActor`))

(event `self.ReceiveBeginPlay`
  ;[1 1 1] Destruir bala a los 3 segundos
  (`KismetSystemLibrary.K2_SetTimerDelegate` (delegate `Destroy`) 3.0))

(event `Destroy`
  ;[1 1 1] Destruir bala a los 3 segundos
  (`self.K2_DestroyActor`))

(event `self.ReceiveTick`
  (params (DeltaSeconds :type "Float (single-precision)"))
  ;[1 1 1] Movimiento de la bala
  (`self.K2_SetActorLocation` (+ (`self.K2_GetActorLocation`) (* (* DeltaSeconds (`self.Speed`)) (`self.GetActorForwardVector`)))))

(fn `UserConstructionScript`)